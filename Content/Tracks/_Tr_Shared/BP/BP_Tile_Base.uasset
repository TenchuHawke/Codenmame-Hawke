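; BP_Tile_Base is, by its name and path, a shared base Blueprint for track tiles that mirrors a path spline into its Spline.
; When PathSpline is valid, the construction script clears Spline and rebuilds it point by point, copying local-space position, tangent and rotation.
; Spline updates are deferred on the add and tangent calls, leaving the rotation call to update.
; The event graph holds no active logic.
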(fn `UserConstructionScript`
  (bind _pathspline (`self.PathSpline`))
  (bind _spline (`self.Spline`))
  (if (`KismetSystemLibrary.IsValid` (`self.PathSpline`))
    (`SplineComponent.ClearSplinePoints` (`self.Spline`) true)
    (for _index (range (`SplineComponent.GetNumberOfSplinePoints` (`self.PathSpline`)))
      (`SplineComponent.AddSplinePoint` _spline (`SplineComponent.GetLocationAtSplinePoint` _pathspline _index "Local") "Local" false)
      (`SplineComponent.SetTangentAtSplinePoint` _spline _index (`SplineComponent.GetTangentAtSplinePoint` _pathspline _index "Local") "Local" false)
      (`SplineComponent.SetRotationAtSplinePoint` _spline _index (`SplineComponent.GetRotationAtSplinePoint` _pathspline _index "Local") "Local" true))))